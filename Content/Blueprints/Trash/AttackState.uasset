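; AttackState is an animation notify state that opens and closes the hit window of an NPC's weapon during an attack animation.
; On begin, it casts the mesh owner to NPC and sets its WeaponBox collision to query only.
; On end, it turns that collision off and prints an "Attacking" debug string.
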(fn `Received_NotifyBegin`
  (params (MeshComp :type "SkeletalMeshComponent Object Reference") (Animation :type "AnimSequenceBase Object Reference") (TotalDuration :type "Float (double-precision)"))
  (returns (ReturnValue :type Boolean))
  (bind _asnpc (cast `/Game/Blueprints/Enemies/NPC` (`ActorComponent.GetOwner` MeshComp)))
  (`PrimitiveComponent.SetCollisionEnabled` (`/Game/Blueprints/Enemies/NPC.WeaponBox` _asnpc) "QueryOnly")
  (return true))

(fn `Received_NotifyEnd`
  (params (MeshComp :type "SkeletalMeshComponent Object Reference") (Animation :type "AnimSequenceBase Object Reference"))
  (returns (ReturnValue :type Boolean))
  (bind _asnpc (cast `/Game/Blueprints/Enemies/NPC` (`ActorComponent.GetOwner` MeshComp)))
  (`PrimitiveComponent.SetCollisionEnabled` (`/Game/Blueprints/Enemies/NPC.WeaponBox` _asnpc) "NoCollision")
  (`KismetSystemLibrary.PrintString` null "Attacking")
  (return false))