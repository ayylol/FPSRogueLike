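; First-person player character that moves, jumps, dashes on a cooldown, fires a shotgun, creates the main HUD and forwards damage to GameMaster.
; Strafe input also rolls the controller to sway the camera up to a limit, easing it level when released.
; Dashing launches along input direction, with a small hop first when grounded.
; Firing triggers the child-actor Weapon and starts Tick-driven recoil, combining camera pitch with a parabolic lerp of the gun's position.
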(event EventBeginPlay
  ;[1 1 1] Draw ui
  (bind _returnvalue (UserInterface|CreateWidget "/Game/Blueprints/MainUI.MainUI_C"))
  (UserInterface|Viewport|AddtoViewport _returnvalue 0))

(event EventTick
  (params (DeltaSeconds :type Float%20%28single-precision%29))
  (bind _camera_recoil_per_sec (Variables|Default|Getcamera_recoil_per_sec))
  (bind _shotgun (Variables|Default|GetShotgun))
  (bind _returnvalue (* DeltaSeconds _camera_recoil_per_sec))
  ;[1 1 1] Gun Recoil
  (if (Variables|Default|Getkick_back)
    (Utilities|Casting|CastToWeapon (Variables|/Script/Engine.ChildActorComponent|GetChildActor _shotgun))
    (if (Variables|Default|Getkick_back_camera)
      (Pawn|Input|AddControllerPitchInput _returnvalue)
      (bind _output_get (Variables|Default|Setrecoil_camera_current (+ _returnvalue (Variables|Default|Getrecoil_camera_current))))
      (Variables|Default|Setkick_back_camera (> _output_get (Variables|Default|Getrecoil_camera_max))))
    (bind _output_get_2 (Variables|Default|Setrecoil_gun_current (+ (* DeltaSeconds (Variables|Default|Getgun_lerp_per_second)) (Variables|Default|Getrecoil_gun_current))))
    (bind _output_get_3 (Variables|Default|Setkick_back_gun (< _output_get_2 1.0)))
    (if _output_get_3
      (Transformation|SetRelativeLocation _shotgun (Math|Vector|Lerp(Vector) (Variables|Default|Getshotgun_default_location) (Variables|Default|Getshotgun_kickback_location) (|(((pow(((2*x)-1),2))*negative)+1) _output_get_2 -1.0)) false false))
    (bind _output_get_4 (Variables|Default|Setkick_back (or (Variables|Default|Getkick_back_camera) (Variables|Default|Getkick_back_gun))))
    (if (not _output_get_4)
      (Transformation|SetRelativeLocation (Variables|Default|GetShotgun) (Variables|Default|Getshotgun_default_location) false false))))

(event Game|Damage|EventAnyDamage
  (params (Damage :type Float%20%28single-precision%29) (DamageType :type Damage%20Type%20Object%20Reference) (InstigatedBy :type Controller%20Object%20Reference) (DamageCauser :type Actor%20Object%20Reference))
  ;[1 1 1] Damage Player
  (bind _returnvalue (Actor|GetActorOfClass "/Game/Blueprints/GameMaster.GameMaster_C"))
  (Default|PlayerDamage _returnvalue Damage))

(event Input|ActionEvents|InputActionDash
  (params (Key :type Key%20Structure :default "None"))
  ;[1 1 1] Dash
  (:Pressed
    (if (Variables|Default|Getcan_dash)
      (if (AI|Components|NavMovement|IsMovingonGround (Pawn|GetMovementComponent))
        (Character|LaunchCharacter "0, 0,200.000000" false false)
        (Utilities|FlowControl|Delay 0.05))
      (Character|LaunchCharacter (* (+ (* (Math|Vector|GetRightVector (Variables|Collision|GetCapsuleComponent)) (Input|AxisValues|GetRight_Left)) (* (Math|Vector|GetForwardVector (Variables|Default|GetFirstPersonCamera)) (Input|AxisValues|GetForward_Backward))) (Variables|Default|Getdash_amount)) false false)
      (Variables|Default|Setcan_dash false)
      (Utilities|FlowControl|Delay (Variables|Default|Getdash_cooldown))
      (Variables|Default|Setcan_dash true))))

(event Input|ActionEvents|InputActionJump
  (params (Key :type Key%20Structure :default "None"))
  ;[1 1 1] Simple Movement
  (:Pressed
    (Character|Jump)))

(event Input|ActionEvents|InputActionFire
  (params (Key :type Key%20Structure :default "None"))
  ;[1 1 1] Shoot weapon
  (:Pressed
    (bind _asweapon (Utilities|Casting|CastToWeapon (Variables|/Script/Engine.ChildActorComponent|GetChildActor (Variables|Default|GetShotgun))))
    (if (Variables|/Game/Blueprints/Weapons/Weapon.Weapon_C|Getcan_shoot _asweapon)
      (Audio|PlaySound2D "/Game/Sounds/shot1.shot1" 1.0 1.0 0.0 0 0)
      (Default|StartShooting _asweapon)
      (Variables|Default|Setrecoil_gun_current 0.0)
      (Variables|Default|Setrecoil_camera_current 0.0)
      (Variables|Default|Setkick_back_gun true)
      (Variables|Default|Setkick_back_camera true)
      (Variables|Default|Setkick_back true))))

(event Input|AxisEvents|InputAxisRotate_Left_Right
  (params (AxisValue :type Float%20%28single-precision%29))
  ;[1 1 1] Simple Movement
  (Pawn|Input|AddControllerYawInput AxisValue))

(event Input|AxisEvents|InputAxisRight_Left
  (params (AxisValue :type Float%20%28single-precision%29))
  (bind _returnvalue (Math|Float|Absolute(Float) AxisValue))
  (bind _firstpersoncamera (Variables|Default|GetFirstPersonCamera))
  (bind _roll_amount_in (Variables|Default|Getroll_amount_in))
  (bind _roll_amount (Variables|Default|Getroll_amount))
  (bind _returnvalue_2 (/ _returnvalue AxisValue))
  (bind _returnvalue_3 (Transformation|GetWorldRotation _firstpersoncamera))
  (bind _roll (Math|Rotator|BreakRotator _returnvalue_3))
  (bind _returnvalue_4 (* _returnvalue_2 _roll_amount))
  (bind _returnvalue_5 (Math|Float|Absolute(Float) _roll))
  (bind _returnvalue_6 (* -1 _roll))
  ;[1 1 1] Camera Sway
  ;;[1 1 1] Check if should be tilting or returning to normal
  (if (Math|Float|NearlyEqual(Float) AxisValue 0.0 0.005)
    ;;[1 1 1] return view to normal
    (if (not (Math|Float|NearlyEqual(Float) _roll 0.0 0.001))
      (if (<= (- _returnvalue_5 _roll_amount_in) _roll_amount_in)
        (Variables|Default|Setroll_to_do _returnvalue_6)
        (else
          (Variables|Default|Setroll_to_do (* _roll_amount_in (/ _returnvalue_5 _returnvalue_6)))))
      ;;[1 1 1] Roll Camera
      (Pawn|Input|AddControllerRollInput (Variables|Default|Getroll_to_do) :!label _label))
    (else
      ;;[1 1 1] sway to side
      (if (<= (* _roll AxisValue) 0.0)
        (Variables|Default|Setroll_to_do (* _returnvalue_2 (Variables|Default|Getroll_amount_in)))
        (goto _label)
        (elif (not (>= (+ (Math|Float|Absolute(Float) _roll) (Math|Float|Absolute(Float) _returnvalue_4)) (Variables|Default|Getmax_roll)))
          (Variables|Default|Setroll_to_do _returnvalue_4)
          (goto _label))))))

(event Input|AxisEvents|InputAxisForward_Backward
  (params (AxisValue :type Float%20%28single-precision%29))
  ;[1 1 1] Simple Movement
  (Pawn|Input|AddMovementInput (Transformation|GetActorForwardVector) AxisValue false))

(event Input|AxisEvents|InputAxisRotate_Up_Down
  (params (AxisValue :type Float%20%28single-precision%29))
  ;[1 1 1] Simple Movement
  (Pawn|Input|AddControllerPitchInput AxisValue))

(event Input|AxisEvents|InputAxisRight_Left
  (params (AxisValue :type Float%20%28single-precision%29))
  ;[1 1 1] Simple Movement
  (Pawn|Input|AddMovementInput (Transformation|GetActorRightVector) AxisValue false))

(fn ConstructionScript
  (bind _output_get (Variables|Default|Setshotgun_default_location (Variables|/Script/Engine.SceneComponent|GetRelativeLocation (Variables|Default|GetShotgun))))
  (Variables|Default|Setshotgun_kickback_location (- _output_get "15.000000, 0, 0")))