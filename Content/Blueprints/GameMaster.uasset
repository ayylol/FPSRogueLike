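; Game master that tracks player health, death/respawn and door-opening on room clear, and populates random rooms via a Q-learning director.
; An epsilon-greedy linear Q-function over 19 state features picks an enemy type or none for each cluster slot.
; The previous room's intensity, from clear time, damage, health and accuracy, is scored against its target to update weights.
; Weights save to QTable.txt, though BeginPlay resets them to 0.5 after loading.
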(event `PlayerDamage`
  (params (Damage :type "Float (double-precision)" :default 0.0))
  (if (`self.CanbeDamaged`)
    (bind _output_get (set `self.PlayerHealth` (- (`self.PlayerHealth`) Damage)))
    (set `self.Currentdamage` (+ Damage (`self.Currentdamage`)))
    (if (<= _output_get 0.0)
      (`self.Death`))))

(event `Death`
  (bind _returnvalue (`|CreateWidget` "/Game/Blueprints/Death.Death_C"))
  (set `self.DeathScreen` _returnvalue)
  (`UserWidget.AddToViewport` _returnvalue 0)
  (set `self.CanbeDamaged` false)
  (bind _returnvalue_2 (`GameplayStatics.GetActorOfClass` "/Game/Blueprints/Door.Door_C"))
  (`/Game/Blueprints/Door.Close` _returnvalue_2)
  (`KismetSystemLibrary.K2_SetTimerDelegate` (delegate `CustomEvent_0`) 5.0))

(event `Enemykilled`
  (bind _result (`/Engine/EditorBlueprintResources/StandardMacros.DecrementInt` (`self.NumEnemies`))
    (:`  `
      (if (<= _result 0)
        (bind _returnvalue (`GameplayStatics.GetActorOfClass` "/Game/Blueprints/Door.Door_C"))
        (`/Game/Blueprints/Door.Open` _returnvalue)
        (else
          (`KismetSystemLibrary.PrintString` (`KismetStringLibrary.Conv_IntToString` _result)))))))

(event `CustomEvent_0`
  (`Widget.RemoveFromParent` (`self.DeathScreen`))
  (bind _returnvalue (`GameplayStatics.GetActorOfClass` "/Game/Blueprints/LevelSpawner.LevelSpawner_C"))
  (set `/Game/Blueprints/LevelSpawner.currentmap` -1 _returnvalue)
  (bind _returnvalue_2 (`GameplayStatics.GetActorOfClass` "/Game/Blueprints/Player.Player_C"))
  (`self.K2_TeleportTo` _returnvalue_2 (-2170.728027 74.995361 238.000366) (struct :`Yaw` -4.602081))
  (bind _returnvalue_3 (`GameplayStatics.GetActorOfClass` "/Game/Blueprints/Triggers/DoorTrigger.DoorTrigger_C"))
  (`/Game/Blueprints/Triggers/DoorTrigger.Triggered` _returnvalue_3 _returnvalue_2)
  (set `self.PlayerHealth` 100.0)
  (set `self.CanbeDamaged` true))

(event `SpawnRoom`
  (bind _returnvalue (`GameplayStatics.GetActorOfClass` "/Game/Blueprints/LevelSpawner.LevelSpawner_C"))
  (`self.SpawnRoomQF` 0.1))

(event `self.ReceiveBeginPlay`
  (`self.LoadQtableFile`)
  (bind _returnvalue (`GameplayStatics.GetActorOfClass` "/Game/Blueprints/LevelSpawner.LevelSpawner_C"))
  (set `/Game/Blueprints/LevelSpawner.currentmap` -1 _returnvalue)
  (`self.SpawnRoom`)
  (for (_ _array_index) (`self.QTable`)
    (`KismetArrayLibrary.Array_Set` (`self.QTable`) _array_index 0.5)))

(event `SpawnRoomQ`)

(fn `BackTrackReward`
  (params (LastState :type "Array of Float (double-precision)"))
  (locals (Numstates :type Integer :default 0) (Rewardnum :type "Float (double-precision)" :default 0.0) (LoopIndex :type Integer :default 0) (Current :type "Array of Float (double-precision)") (Next :type "Array of Float (double-precision)"))
  (bind _numstates (`local.Numstates`))
  (bind _returnvalue (`KismetArrayLibrary.Array_Length` (`self.Statehistory`)))
  (bind _returnvalue_2 (* (`local.LoopIndex`) 19))
  (bind _returnvalue_3 (/ _returnvalue 19))
  (bind _returnvalue_4 (* (+ (`local.LoopIndex`) 1) 19))
  (if (not (== _returnvalue_3 (`KismetArrayLibrary.Array_Length` (`self.ActionHistory`))))
    (`KismetSystemLibrary.PrintString` "Mismatched Action and State Histories"))
  (if (== _returnvalue 0)
    (return)
    (else
      (set `local.Numstates` (- _returnvalue_3 1))
      (bind _reward (`self.Reward`))
      (set `local.Rewardnum` _reward)
      (for _index (range (+ _numstates 1))
        (bind _output_get (set `local.LoopIndex` _index))
        (`KismetArrayLibrary.Array_Clear` (`local.Current`))
        (for _index_2 (range _returnvalue_2 (+ (+ _returnvalue_2 18) 1))
          (`KismetArrayLibrary.Array_Add` (`local.Current`) (`|GetArrayItem` (`self.Statehistory`) _index_2)))
        (if (== _output_get _numstates)
          (bind _returnvalue_5 (* (/ (`KismetMathLibrary.Conv_IntToDouble` _index) (`KismetMathLibrary.Conv_IntToDouble` _numstates)) (`local.Rewardnum`)))
          (`self.UpdateQTable` (`|GetArrayItem` (`self.ActionHistory`) (`local.LoopIndex`)) _returnvalue_5 (`local.Current`) LastState)
          (else
            (`KismetArrayLibrary.Array_Clear` (`local.Next`))
            (for _index_3 (range _returnvalue_4 (+ (+ _returnvalue_4 18) 1))
              (`KismetArrayLibrary.Array_Add` (`local.Next`) (`|GetArrayItem` (`self.Statehistory`) _index_3)))
            (`self.UpdateQTable` (`|GetArrayItem` (`self.ActionHistory`) (`local.LoopIndex`)) _returnvalue_5 (`local.Current`) (`local.Next`)))))
      (`KismetArrayLibrary.Array_Clear` (`self.Statehistory`))
      (`KismetArrayLibrary.Array_Clear` (`self.ActionHistory`))
      (`self.WriteToQtableFile`))))

(fn `CalcIntensity`
  (params (Cleartime :type "Float (double-precision)") (DamageTaken :type "Float (double-precision)") (HealthAtEnd :type "Float (double-precision)") (Accuracy :type "Float (double-precision)") (NumEnemies :type Integer))
  (returns (Intensity :type "Float (double-precision)"))
  (locals (NewLocalVar_0 :type Integer) (NewLocalVar_1 :type Integer))
  (bind _returnvalue (* Accuracy 0.3))
  (bind _returnvalue_2 (* (/ DamageTaken 100.0) 0.4))
  (bind _returnvalue_3 (/ (/ Cleartime (`KismetMathLibrary.Conv_IntToDouble` NumEnemies)) 20.0))
  (bind _returnvalue_4 (* (- 1.0 (/ HealthAtEnd 100.0)) 0.2))
  (if (> _returnvalue_3 1.0)
    (return (+ 0.0 _returnvalue_2 _returnvalue_4 _returnvalue))
    (else
      (return (+ (* (- 1.0 _returnvalue_3) 0.1) _returnvalue_2 _returnvalue_4 _returnvalue)))))

(fn `GetQ`
  (params (State :type "Array of Float (double-precision)") (Action :type Integer))
  (returns (Qval :type "Float (double-precision)"))
  (locals (QValue :type "Float (double-precision)"))
  (bind _returnvalue (* Action 19))
  (bind _qtable (`self.QTable`))
  (set `local.QValue` (`|GetArrayItem` _qtable _returnvalue)) ; initially set the always 1 weight
  (for (_array_element _array_index) State
    (set `local.QValue` (+ (* _array_element (`|GetArrayItem` _qtable (+ _array_index _returnvalue))) (`local.QValue`))))
  (return (`local.QValue`)))

(fn `LoadQtableFile`
  (for (_array_element _array_index) (`VictoryBPFunctionLibrary.LoadStringArrayFromFile` (`KismetStringLibrary.Concat_StrStr` (`KismetStringLibrary.Concat_StrStr` (`VictoryBPFunctionLibrary.VictoryPaths__GameRootDirectory`) "Content/") (`self.filename`)))
    (`KismetArrayLibrary.Array_Set` (`self.QTable`) _array_index (`KismetStringLibrary.Conv_StringToDouble` _array_element) true)))

(fn `Perform Action+ Observe Next Step`
  (params (Action :type Integer))
  ;[1 1 1] This is where you hook it up to enemy generation. Five actions (0-4) represent different enemy types?
)

(fn `Reward`
  (returns (Reward :type "Float (double-precision)"))
  (bind _returnvalue (`KismetMathLibrary.Abs` (- (`self.HistoricalTargertIntensity`) (`self.Intensity`))))
  (bind _returnvalue_2 (* _returnvalue (`self.RewardMax`)))
  (bind _returnvalue_3 (* _returnvalue_2 -1.0))
  (if (< _returnvalue 0.3)
    (`KismetSystemLibrary.PrintString` (`KismetStringLibrary.Conv_DoubleToString` _returnvalue_2))
    (return _returnvalue_2)
    (else
      (`KismetSystemLibrary.PrintString` (`KismetStringLibrary.Conv_DoubleToString` _returnvalue_3))
      (return _returnvalue_3))))

(fn `SelectAction`
  (params (State :type "Array of Float (double-precision)"))
  (returns (Action :type Integer))
  (if (< (`KismetMathLibrary.RandomInteger` 10) 9)
    (bind _qval (`self.GetQ` State))
    (bind _qval_2 (`self.GetQ` State 1))
    (bind _qval_3 (`self.GetQ` State 2))
    (bind _qval_4 (`self.GetQ` State 3))
    (bind _qval_5 (`self.GetQ` State 4))
    (return (`KismetMathLibrary.MaxOfFloatArray` (`|MakeArray` _qval _qval_2 _qval_3 _qval_4 _qval_5)))
    (else
      (`KismetSystemLibrary.PrintString` "Random")
      (return (`KismetMathLibrary.RandomInteger` 5)))))

(fn `SetWeightQ`
  (params (FeatureIndex :type Integer) (Action :type Integer) (Weight :type "Float (double-precision)"))
  (bind _qtable (`self.QTable`))
  (bind _returnvalue (+ FeatureIndex (* Action 19)))
  (bind _returnvalue_2 (+ Weight (`|GetArrayItem` _qtable _returnvalue)))
  (`KismetArrayLibrary.Array_Set` _qtable _returnvalue _returnvalue_2)
  (if (== _returnvalue 0)
    (`KismetSystemLibrary.PrintString` (`KismetStringLibrary.Conv_DoubleToString` _returnvalue_2)))
  (return))

(fn `SpawnRoomQF`
  (params (TargetIntensity :type "Float (double-precision)"))
  (locals (TargetRoom :type Integer :default 0) (LocalStateMaps :type "Array of Float (double-precision)") (LocalStateCluster :type "Array of Float (double-precision)") (EnemiesinRoom :type Integer) (EnemiesinCluster :type Integer) (LocalState :type "Array of Float (double-precision)") (LevelS :type "/Game/Blueprints/LevelSpawner Object Reference"))
  (`self.StartEndRoomVariables`)
  (bind _output_get (set `local.TargetRoom` (`KismetMathLibrary.RandomIntegerInRange` 0 9)))
  (for _ (range _output_get)
    (`KismetArrayLibrary.Array_Add` (`local.LocalStateMaps`)))
  (`KismetArrayLibrary.Array_Add` (`local.LocalStateMaps`) 1.0)
  (while (< (`KismetArrayLibrary.Array_Length` (`local.LocalStateMaps`)) 10)
    (`KismetArrayLibrary.Array_Add` (`local.LocalStateMaps`)))
  (bind _returnvalue (`GameplayStatics.GetActorOfClass` "/Game/Blueprints/LevelSpawner.LevelSpawner_C"))
  (set `local.LevelS` _returnvalue)
  (`/Game/Blueprints/LevelSpawner.Spawnmap` _returnvalue _output_get)
  (for _index (range 4)
    (set `local.EnemiesinCluster` 0)
    (`KismetArrayLibrary.Array_Clear` (`local.LocalStateCluster`))
    (for _ (range _index)
      (`KismetArrayLibrary.Array_Add` (`local.LocalStateCluster`)))
    (`KismetArrayLibrary.Array_Add` (`local.LocalStateCluster`) 1.0)
    (while (< (`KismetArrayLibrary.Array_Length` (`local.LocalStateCluster`)) 4)
      (`KismetArrayLibrary.Array_Add` (`local.LocalStateCluster`)))
    (for _index_2 (range 1 (+ (`self.MaxEnemyPerCluster`) 1))
      (`KismetArrayLibrary.Array_Clear` (`local.LocalState`))
      (`KismetArrayLibrary.Array_Add` (`local.LocalState`) 1.0)
      (`KismetArrayLibrary.Array_Append` (`local.LocalState`) (`local.LocalStateMaps`))
      (`KismetArrayLibrary.Array_Append` (`local.LocalState`) (`local.LocalStateCluster`))
      (`KismetArrayLibrary.Array_Add` (`local.LocalState`) (/ (`KismetMathLibrary.Conv_IntToDouble` (`local.EnemiesinCluster`)) (`KismetMathLibrary.Conv_IntToDouble` (`self.MaxEnemyPerCluster`))))
      (`KismetArrayLibrary.Array_Add` (`local.LocalState`) (/ (`KismetMathLibrary.Conv_IntToDouble` (`local.EnemiesinRoom`)) (`KismetMathLibrary.Conv_IntToDouble` (* (`self.MaxEnemyPerCluster`) 4))))
      (`KismetArrayLibrary.Array_Add` (`local.LocalState`) TargetIntensity)
      (`KismetArrayLibrary.Array_Add` (`local.LocalState`) (/ (`KismetMathLibrary.Conv_IntToDouble` _index_2) (`KismetMathLibrary.Conv_IntToDouble` (`self.MaxEnemyPerCluster`))))
      (if (and (== _index 0) (== _index_2 1))
        (`self.BackTrackReward` (`local.LocalState`)))
      (bind _action (`self.SelectAction` (`local.LocalState`)))
      (if (!= _action 4)
        (`/Game/Blueprints/LevelSpawner.SpawnEnemiesInput` (`local.LevelS`) _index _index_2 _action)
        (`/Engine/EditorBlueprintResources/StandardMacros.IncrementInt` (`local.EnemiesinRoom`)
          (:`  `
            (`/Engine/EditorBlueprintResources/StandardMacros.IncrementInt` (`local.EnemiesinCluster`)
              (:`  `
                _)))))
      (`KismetArrayLibrary.Array_Append` (`self.Statehistory`) (`local.LocalState`))
      (`KismetArrayLibrary.Array_Add` (`self.ActionHistory`) _action)))
  (bind _output_get_2 (set `self.NumEnemies` (`local.EnemiesinRoom`)))
  (set `self.HistoricalTargertIntensity` TargetIntensity))

(fn `StartEndRoomVariables`
  (bind _returnvalue (`GameplayStatics.GetTimeSeconds`))
  (bind _roomstarttime (`self.RoomstartTime`))
  (if (!= _roomstarttime _returnvalue)
    (bind _output_get (set `self.Cleartime` (- _returnvalue _roomstarttime)))
    (for _array_element (`self.GetAllChildActors` (`GameplayStatics.GetPlayerCharacter` 0) true)
      (if (`KismetMathLibrary.ClassIsChildOf` (`GameplayStatics.GetObjectClass` _array_element) "/Game/Blueprints/Weapons/Weapon.Weapon_C")
        (bind _asweapon (cast `/Game/Blueprints/Weapons/Weapon` _array_element))
        (bind _intensity (`self.CalcIntensity` _output_get (`self.Currentdamage`) (`self.PlayerHealth`) (`/Game/Blueprints/Weapons/Weapon.current_accuracy` _asweapon) (`self.NumEnemies`)))
        (bind _output_get_2 (set `self.Intensity` _intensity))
        (`KismetSystemLibrary.PrintString` (`KismetStringLibrary.Conv_DoubleToString` _output_get_2))
        (if (< (`self.Cleartime`) 30.0)
          (set `self.PlayerHealth` (+ (* (* (/ (`self.Cleartime`) 30.0) 0.75) (`self.Currentdamage`)) (`self.PlayerHealth`))))
        (set `self.RoomstartTime` _returnvalue :!label _label)
        (set `self.Currentdamage` 0.0)
        (set `self.NumEnemies` 0)))
    (else
      (goto _label))))

(fn `UpdateQTable`
  (params (Action :type Integer) (Reward :type "Float (double-precision)") (State :type "Array of Float (double-precision)") (NextState :type "Array of Float (double-precision)"))
  (bind _qval (`self.GetQ` State Action))
  (bind _qval_2 (`self.GetQ` NextState))
  (bind _qval_3 (`self.GetQ` NextState 1))
  (bind _qval_4 (`self.GetQ` NextState 2))
  (bind _qval_5 (`self.GetQ` NextState 3))
  (bind _qval_6 (`self.GetQ` NextState 4))
  (bind _returnvalue (* (`self.Alpha`) (+ (- (* 0.3 (`KismetMathLibrary.FMax` _qval_2 _qval_3 _qval_4 _qval_5 _qval_6)) _qval) Reward)))
  (`self.SetWeightQ` 0 Action _returnvalue) ; Update always1
  (for (_array_element _array_index) State
    (if (> _array_element 0.0)
      (`self.SetWeightQ` _array_index Action _returnvalue) ; only update if feature is nonzero
    ))
  (`KismetSystemLibrary.PrintString` "QTable -- Updated weights"))

(fn `UpdateState`
  (set `self.State` (`self.NextState`)))

(fn `UserConstructionScript`)

(fn `WriteToQtableFile`
  (bind _qtable_string (`self.Qtable_String`))
  (`KismetArrayLibrary.Array_Clear` _qtable_string)
  (for _array_element (`self.QTable`)
    (`KismetArrayLibrary.Array_Add` _qtable_string (`KismetStringLibrary.Conv_DoubleToString` _array_element)))
  (`VictoryBPFunctionLibrary.FileIO__SaveStringArrayToFile` (`KismetStringLibrary.Concat_StrStr` (`VictoryBPFunctionLibrary.VictoryPaths__GameRootDirectory`) "Content/") "QTable.txt" (`self.Qtable_String`) true))