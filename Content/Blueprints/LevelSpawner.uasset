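; LevelSpawner swaps arena maps, spawns their enemies and opens the exit Door once all are killed.
; Spawnmap destroys existing Map and NPC actors before spawning one of four map Blueprints at origin; SpawnOrdered cycles through them.
; SpawnEnemies fills four quadrant grids of up to nine slots each with chained switch cases, one NPC class per quadrant.
; It stores the total, which Enemykilled decrements until the Door opens.
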(event `Spawnmap`
  (params (Map :type Integer))
  (bind _returnvalue (`KismetMathLibrary.MakeTransform` (0.0 0.0 0.0)))
  (set `self.#enemies` 0)
  (bind _outactors (`GameplayStatics.GetAllActorsOfClass` "/Game/Blueprints/Map/Map.Map_C"))
  (for _array_element _outactors
    (`self.K2_DestroyActor` _array_element))
  (bind _outactors_2 (`GameplayStatics.GetAllActorsOfClass` "/Game/Blueprints/Enemies/NPC.NPC_C"))
  (for _array_element_2 _outactors_2
    (`self.K2_DestroyActor` _array_element_2))
  (switch `int` Map
    (:`0`
      (`|SpawnActorFromClass` "/Game/Blueprints/Map/StageAndPodium_Blueprint.StageAndPodium_Blueprint_C" _returnvalue "Undefined" "OverrideRootScale" null null))
    (:`1`
      (`|SpawnActorFromClass` "/Game/Blueprints/Map/TreeHouse_Blueprint.TreeHouse_Blueprint_C" _returnvalue "Undefined" "OverrideRootScale" null null))
    (:`2`
      (`|SpawnActorFromClass` "/Game/Blueprints/Map/Dipped_Blueprint.Dipped_Blueprint_C" _returnvalue "Undefined" "OverrideRootScale" null null))
    (:`3`
      (`|SpawnActorFromClass` "/Game/Blueprints/Map/SkyScraper_Blueprint.SkyScraper_Blueprint_C" _returnvalue "Undefined" "OverrideRootScale" null null))))

(event `Enemykilled`
  (bind _result (`/Engine/EditorBlueprintResources/StandardMacros.DecrementInt` (`self.#enemies`))
    (:`  `
      (if (<= _result 0)
        (bind _returnvalue (`GameplayStatics.GetActorOfClass` "/Game/Blueprints/Door.Door_C"))
        (`/Game/Blueprints/Door.Open` _returnvalue)
        (else
          (`KismetSystemLibrary.PrintString` (`KismetStringLibrary.Conv_IntToString` _result)))))))

(event `SpawnOrdered`
  (bind _result (`/Engine/EditorBlueprintResources/StandardMacros.IncrementInt` (`self.currentmap`))
    (:`  `
      (if (> _result (`self.maxmap`))
        (set `self.currentmap` 0))
      (`self.Spawnmap` (`self.currentmap`)))))

(event `SpawnEnemies`
  (params (Block1 :type Integer) (Block2 :type Integer) (Block3 :type Integer) (Block4 :type Integer) (NPC1 :type "Actor Class Reference") (NPC2 :type "Actor Class Reference") (NPC3 :type "Actor Class Reference") (NPC4 :type "Actor Class Reference"))
  (switch `int` Block1
    (:`Default`
      _)
    (:`0`
      _)
    (:`1`
      (`|SpawnActorFromClass` NPC1 (`KismetMathLibrary.MakeTransform` (700.0 700.0 2500.0)) "Undefined" "OverrideRootScale" null null :!label _label))
    (:`2`
      (`|SpawnActorFromClass` NPC1 (`KismetMathLibrary.MakeTransform` (700.0 1000.0 2500.0)) "Undefined" "OverrideRootScale" null null :!label _label_2)
      (goto _label))
    (:`3`
      (`|SpawnActorFromClass` NPC1 (`KismetMathLibrary.MakeTransform` (700.0 1300.0 2500.0)) "Undefined" "OverrideRootScale" null null :!label _label_3)
      (goto _label_2))
    (:`4`
      (`|SpawnActorFromClass` NPC1 (`KismetMathLibrary.MakeTransform` (1000.0 700.0 2500.0)) "Undefined" "OverrideRootScale" null null :!label _label_4)
      (goto _label_3))
    (:`5`
      (`|SpawnActorFromClass` NPC1 (`KismetMathLibrary.MakeTransform` (1000.0 1000.0 2500.0)) "Undefined" "OverrideRootScale" null null :!label _label_5)
      (goto _label_4))
    (:`6`
      (`|SpawnActorFromClass` NPC1 (`KismetMathLibrary.MakeTransform` (1000.0 1300.0 2500.0)) "Undefined" "OverrideRootScale" null null :!label _label_6)
      (goto _label_5))
    (:`7`
      (`|SpawnActorFromClass` NPC1 (`KismetMathLibrary.MakeTransform` (1300.0 700.0 2500.0)) "Undefined" "OverrideRootScale" null null :!label _label_7)
      (goto _label_6))
    (:`8`
      (`|SpawnActorFromClass` NPC1 (`KismetMathLibrary.MakeTransform` (1300.0 1000.0 2500.0)) "Undefined" "OverrideRootScale" null null :!label _label_8)
      (goto _label_7))
    (:`9`
      (`|SpawnActorFromClass` NPC1 (`KismetMathLibrary.MakeTransform` (1300.0 1300.0 2500.0)) "Undefined" "OverrideRootScale" null null)
      (goto _label_8)))
  (switch `int` Block2
    (:`Default`
      _)
    (:`0`
      _)
    (:`1`
      (`|SpawnActorFromClass` NPC2 (`KismetMathLibrary.MakeTransform` (-700.0 700.0 2500.0)) "Undefined" "OverrideRootScale" null null :!label _label_9))
    (:`2`
      (`|SpawnActorFromClass` NPC2 (`KismetMathLibrary.MakeTransform` (-700.0 1000.0 2500.0)) "Undefined" "OverrideRootScale" null null :!label _label_10)
      (goto _label_9))
    (:`3`
      (`|SpawnActorFromClass` NPC2 (`KismetMathLibrary.MakeTransform` (-700.0 1300.0 2500.0)) "Undefined" "OverrideRootScale" null null :!label _label_11)
      (goto _label_10))
    (:`4`
      (`|SpawnActorFromClass` NPC2 (`KismetMathLibrary.MakeTransform` (-1000.0 700.0 2500.0)) "Undefined" "OverrideRootScale" null null :!label _label_12)
      (goto _label_11))
    (:`5`
      (`|SpawnActorFromClass` NPC2 (`KismetMathLibrary.MakeTransform` (-1000.0 1000.0 2500.0)) "Undefined" "OverrideRootScale" null null :!label _label_13)
      (goto _label_12))
    (:`6`
      (`|SpawnActorFromClass` NPC2 (`KismetMathLibrary.MakeTransform` (-1000.0 1300.0 2500.0)) "Undefined" "OverrideRootScale" null null :!label _label_14)
      (goto _label_13))
    (:`7`
      (`|SpawnActorFromClass` NPC2 (`KismetMathLibrary.MakeTransform` (-1300.0 700.0 2500.0)) "Undefined" "OverrideRootScale" null null :!label _label_15)
      (goto _label_14))
    (:`8`
      (`|SpawnActorFromClass` NPC2 (`KismetMathLibrary.MakeTransform` (-1300.0 1000.0 2500.0)) "Undefined" "OverrideRootScale" null null :!label _label_16)
      (goto _label_15))
    (:`9`
      (`|SpawnActorFromClass` NPC2 (`KismetMathLibrary.MakeTransform` (-1300.0 1300.0 2500.0)) "Undefined" "OverrideRootScale" null null)
      (goto _label_16)))
  (switch `int` Block3
    (:`Default`
      _)
    (:`0`
      _)
    (:`1`
      (`|SpawnActorFromClass` NPC3 (`KismetMathLibrary.MakeTransform` (-700.0 -700.0 2500.0)) "Undefined" "OverrideRootScale" null null :!label _label_17))
    (:`2`
      (`|SpawnActorFromClass` NPC3 (`KismetMathLibrary.MakeTransform` (-700.0 -1000.0 2500.0)) "Undefined" "OverrideRootScale" null null :!label _label_18)
      (goto _label_17))
    (:`3`
      (`|SpawnActorFromClass` NPC3 (`KismetMathLibrary.MakeTransform` (-700.0 -1300.0 2500.0)) "Undefined" "OverrideRootScale" null null :!label _label_19)
      (goto _label_18))
    (:`4`
      (`|SpawnActorFromClass` NPC3 (`KismetMathLibrary.MakeTransform` (-1000.0 -700.0 2500.0)) "Undefined" "OverrideRootScale" null null :!label _label_20)
      (goto _label_19))
    (:`5`
      (`|SpawnActorFromClass` NPC3 (`KismetMathLibrary.MakeTransform` (-1000.0 -1000.0 2500.0)) "Undefined" "OverrideRootScale" null null :!label _label_21)
      (goto _label_20))
    (:`6`
      (`|SpawnActorFromClass` NPC3 (`KismetMathLibrary.MakeTransform` (-1000.0 -1300.0 2500.0)) "Undefined" "OverrideRootScale" null null :!label _label_22)
      (goto _label_21))
    (:`7`
      (`|SpawnActorFromClass` NPC3 (`KismetMathLibrary.MakeTransform` (-1300.0 -700.0 2500.0)) "Undefined" "OverrideRootScale" null null :!label _label_23)
      (goto _label_22))
    (:`8`
      (`|SpawnActorFromClass` NPC3 (`KismetMathLibrary.MakeTransform` (-1300.0 -1000.0 2500.0)) "Undefined" "OverrideRootScale" null null :!label _label_24)
      (goto _label_23))
    (:`9`
      (`|SpawnActorFromClass` NPC3 (`KismetMathLibrary.MakeTransform` (-1300.0 -1300.0 2500.0)) "Undefined" "OverrideRootScale" null null)
      (goto _label_24)))
  (switch `int` Block4
    (:`Default`
      _)
    (:`0`
      _)
    (:`1`
      (`|SpawnActorFromClass` NPC4 (`KismetMathLibrary.MakeTransform` (700.0 -700.0 2500.0)) "Undefined" "OverrideRootScale" null null :!label _label_25))
    (:`2`
      (`|SpawnActorFromClass` NPC4 (`KismetMathLibrary.MakeTransform` (700.0 -1000.0 2500.0)) "Undefined" "OverrideRootScale" null null :!label _label_26)
      (goto _label_25))
    (:`3`
      (`|SpawnActorFromClass` NPC4 (`KismetMathLibrary.MakeTransform` (700.0 -1300.0 2500.0)) "Undefined" "OverrideRootScale" null null :!label _label_27)
      (goto _label_26))
    (:`4`
      (`|SpawnActorFromClass` NPC4 (`KismetMathLibrary.MakeTransform` (1000.0 -700.0 2500.0)) "Undefined" "OverrideRootScale" null null :!label _label_28)
      (goto _label_27))
    (:`5`
      (`|SpawnActorFromClass` NPC4 (`KismetMathLibrary.MakeTransform` (1000.0 -1000.0 2500.0)) "Undefined" "OverrideRootScale" null null :!label _label_29)
      (goto _label_28))
    (:`6`
      (`|SpawnActorFromClass` NPC4 (`KismetMathLibrary.MakeTransform` (1000.0 -1300.0 2500.0)) "Undefined" "OverrideRootScale" null null :!label _label_30)
      (goto _label_29))
    (:`7`
      (`|SpawnActorFromClass` NPC4 (`KismetMathLibrary.MakeTransform` (1300.0 -700.0 2500.0)) "Undefined" "OverrideRootScale" null null :!label _label_31)
      (goto _label_30))
    (:`8`
      (`|SpawnActorFromClass` NPC4 (`KismetMathLibrary.MakeTransform` (1300.0 -1000.0 2500.0)) "Undefined" "OverrideRootScale" null null :!label _label_32)
      (goto _label_31))
    (:`9`
      (`|SpawnActorFromClass` NPC4 (`KismetMathLibrary.MakeTransform` (1300.0 -1300.0 2500.0)) "Undefined" "OverrideRootScale" null null)
      (goto _label_32)))
  (set `self.#enemies` (+ Block1 Block2 Block3 Block4)))

(fn `UserConstructionScript`)