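; Weapon Blueprint attached to a Player as a child actor, firing in either hitscan or projectile mode.
; StartShooting fires all shots in one burst, then blocks firing for the rate-of-fire delay.
; Hitscan traces from the first-person camera with random spread that grows per shot, draws debug lines and calls Shot on hit NPCs.
; Projectile mode spawns Bullets at the fire point using unspread camera rotation.
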(event `StartShooting`
  (if (`self.can_shoot`)
    (bind _asplayer (cast `/Game/Blueprints/Player` (`self.GetParentActor` self)))
    (set `self.current_accuracy` (`self.first_shot_accuracy`))
    (while (< (`self.shots_fired`) (`self.projectiles_per_shot`))
      (if (`self.is_hitscan`)
        (bind _firstpersoncamera (`/Game/Blueprints/Player.FirstPersonCamera` _asplayer))
        (bind _returnvalue (`SceneComponent.K2_GetComponentRotation` _firstpersoncamera))
        (`self.ShootLaser` (`SceneComponent.K2_GetComponentLocation` _firstpersoncamera) (`KismetMathLibrary.ComposeRotators` (* (`KismetMathLibrary.RandomRotator` false) (`self.current_accuracy`)) _returnvalue) _asplayer)
        (else
          (`self.Shoot` (`SceneComponent.K2_GetComponentLocation` (`/Game/Blueprints/Player.FirePoint` _asplayer)) _returnvalue)))
      (set `self.shots_fired` (+ (`self.shots_fired`) 1))
      (set `self.current_accuracy` (+ (`self.current_accuracy`) (`self.accuracy_loss`))))
    (set `self.can_shoot` false)
    (`KismetSystemLibrary.Delay` (`self.rate_of_fire`))
    (set `self.can_shoot` true)
    (set `self.shots_fired` 0)))

(fn `Shoot`
  (params (ShotLocation :type "Vector Structure") (CameraRotation :type "Rotator Structure"))
  (`|SpawnActorFromClass` (`self.Bullet`) (`KismetMathLibrary.MakeTransform` ShotLocation CameraRotation) "Undefined" "OverrideRootScale" null null))

(fn `ShootLaser`
  (params (Start :type "Vector Structure") (Rotation :type "Rotator Structure") (shooter :type "Actor Object Reference"))
  (bind _outhit (`KismetSystemLibrary.LineTraceSingleForObjects` Start (+ Start (* (`KismetMathLibrary.GetForwardVector` Rotation) 3000.0)) (`self.Object Types`) false (`|MakeArray` shooter) "ForDuration" true (struct :`R` 1.0 :`G` 0.690805 :`A` 1.0) (struct :`R` 0.924611 :`G` 0.927083 :`B` 0.883895 :`A` 0.005) 0.2))
  (bind _asnpc (cast `/Game/Blueprints/Enemies/NPC` (`.HitActor` (`GameplayStatics.BreakHitResult` _outhit))))
  (`/Game/Blueprints/Enemies/NPC.Shot` _asnpc))

(fn `UserConstructionScript`)