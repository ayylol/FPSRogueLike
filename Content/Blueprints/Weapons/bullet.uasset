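; Bullet projectile actor that destroys itself when it overlaps a target or hits an obstacle.
; The construction script feeds ProjectileSpeed into the projectile movement's max and initial speed.
; Box overlaps ignore actors of the Shooter's class and other bullets, while blocking hits always destroy it.
; Each event only prints a debug string, with no damage applied.
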(event `self.Box.OnComponentBeginOverlap`
  (params (OverlappedComponent :type "PrimitiveComponent Object Reference") (OtherActor :type "Actor Object Reference") (OtherComp :type "PrimitiveComponent Object Reference") (OtherBodyIndex :type Integer) (bFromSweep :type Boolean) (SweepResult :type "HitResult Structure (by ref)"))
  (bind _returnvalue (`GameplayStatics.GetObjectClass` OtherActor))
  (if (and (!= (`self.shooter`) _returnvalue) (!= _returnvalue (`GameplayStatics.GetObjectClass` self)))
    (`KismetSystemLibrary.PrintString` "Shot")
    (`self.K2_DestroyActor` :!label _label)))

(event `self.ReceiveHit`
  (params (MyComp :type "PrimitiveComponent Object Reference") (Other :type "Actor Object Reference") (OtherComp :type "PrimitiveComponent Object Reference") (bSelfMoved :type Boolean) (HitLocation :type "Vector Structure") (HitNormal :type "Vector Structure") (NormalImpulse :type "Vector Structure") (Hit :type "HitResult Structure (by ref)"))
  (`KismetSystemLibrary.PrintString` "HitObstacle")
  (goto _label))

(event `self.ReceiveBeginPlay`
  (`KismetSystemLibrary.PrintString` "spawned"))

(fn `UserConstructionScript`
  (bind _projectilemovement (`self.ProjectileMovement`))
  (bind _output_get (set `ProjectileMovementComponent.MaxSpeed` (`self.projectile_speed`) _projectilemovement))
  (set `ProjectileMovementComponent.InitialSpeed` _output_get _projectilemovement))