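; Weapon projectile actor that shoots NPCs it overlaps and destroys itself on impact.
; The construction script sets the ProjectileMovement velocity along X from ProjectileSpeed.
; Overlaps skip the Shooter's class, other projectiles of its class and DoorCloseTrigger; NPCs or their subclasses receive Shot before the projectile is destroyed.
; Hit events also destroy it, and debug strings print on spawn, overlap, shot and obstacle hit.
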(event `self.ReceiveActorBeginOverlap`
  (params (OtherActor :type "Actor Object Reference"))
  (bind _returnvalue (`GameplayStatics.GetObjectClass` OtherActor))
  (bind _returnvalue_2 (`GameplayStatics.GetObjectClass` OtherActor))
  (`KismetSystemLibrary.PrintString` "Overlap")
  (if (and (!= (`self.shooter`) _returnvalue_2) (!= _returnvalue_2 (`GameplayStatics.GetObjectClass` self)) (!= _returnvalue_2 "/Game/Blueprints/Triggers/DoorCloseTrigger.DoorCloseTrigger_C"))
    (if (or (== _returnvalue "/Game/Blueprints/NPC.NPC_C") (`KismetMathLibrary.ClassIsChildOf` _returnvalue "/Game/Blueprints/NPC.NPC_C"))
      (bind _asnpc (cast `/Game/Blueprints/NPC` OtherActor))
      (`/Game/Blueprints/NPC.Shot` _asnpc)
      (`KismetSystemLibrary.PrintString` "Shot")
      (`self.K2_DestroyActor` :!label _label))))

(event `self.ReceiveHit`
  (params (MyComp :type "PrimitiveComponent Object Reference") (Other :type "Actor Object Reference") (OtherComp :type "PrimitiveComponent Object Reference") (bSelfMoved :type Boolean) (HitLocation :type "Vector Structure") (HitNormal :type "Vector Structure") (NormalImpulse :type "Vector Structure") (Hit :type "HitResult Structure (by ref)"))
  (`KismetSystemLibrary.PrintString` "HitObstacle")
  (goto _label))

(event `self.ReceiveBeginPlay`
  (`KismetSystemLibrary.PrintString` "spawned"))

(fn `UserConstructionScript`
  (set `MovementComponent.Velocity` (`KismetMathLibrary.MakeVector` (`self.projectile_speed`)) (`self.ProjectileMovement`)))