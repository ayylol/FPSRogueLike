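; Door actor that slides its static mesh vertically between hard-coded closed and raised relative positions.
; On BeginPlay it moves to closed, then a one-shot timer opens it after five seconds.
; Close and Open events drive MoveComponentTo, and Toggle alternates between them using the Isopen flag.
; Only Toggle updates that flag, so the timed opening leaves it unchanged.
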(event `self.ReceiveBeginPlay`
  (`self.Close`)
  (`KismetSystemLibrary.K2_SetTimerDelegate` (delegate `OpenDoor`) 5.0))

(event `OpenDoor`
  (`self.Open`))

(event `Close`
  (`KismetSystemLibrary.MoveComponentTo` (`self.StaticMeshComponent`) (-1520.0 10.0 300.0)))

(event `Open`
  (`KismetSystemLibrary.MoveComponentTo` (`self.StaticMeshComponent`) (-1520.0 10.0 900.0)))

(event `Toggle`
  (if (`self.isopen`)
    (`self.Close`)
    (set `self.isopen` false)
    (else
      (`self.Open`)
      (set `self.isopen` true))))

(fn `UserConstructionScript`)