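; Player trigger that runs a door cycle to spawn a new room through the GameMaster.
; Overlap or the Triggered event, if the actor is the Player and the trigger is Active, disarms it and closes the Door.
; After timed delays it calls SpawnRoom, reopens the Door and arms the DoorCloseTrigger; SetActive re-arms this trigger.
; Door, GameMaster and DoorCloseTrigger are found by class lookup, not stored references.
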(event `Triggered`
  (params (`Other Actor` :type "Actor Object Reference"))
  (if (and (== (`GameplayStatics.GetObjectClass` `Other Actor`) "/Game/Blueprints/Player.Player_C") (`self.active`))
    (set `self.active` false :!label _label)
    (bind _returnvalue (`GameplayStatics.GetActorOfClass` "/Game/Blueprints/Door.Door_C"))
    (bind _asdoor (cast `/Game/Blueprints/Door` _returnvalue))
    (`/Game/Blueprints/Door.Close` _asdoor)
    (`KismetSystemLibrary.Delay` 2.0)
    (bind _returnvalue_2 (`GameplayStatics.GetActorOfClass` "/Game/Blueprints/GameMaster.GameMaster_C"))
    (`/Game/Blueprints/GameMaster.SpawnRoom` _returnvalue_2)
    (`KismetSystemLibrary.Delay` 2.0)
    (`/Game/Blueprints/Door.Open` _asdoor)
    (bind _returnvalue_3 (`GameplayStatics.GetActorOfClass` "/Game/Blueprints/Triggers/DoorCloseTrigger.DoorCloseTrigger_C"))
    (`/Game/Blueprints/Triggers/DoorCloseTrigger.SetActive` _returnvalue_3)))

(event `self.ReceiveActorBeginOverlap`
  (params (OtherActor :type "Actor Object Reference"))
  (if (and (== (`GameplayStatics.GetObjectClass` OtherActor) "/Game/Blueprints/Player.Player_C") (`self.active`))
    (goto _label)))

(event `SetActive`
  (set `self.active` true))

(fn `UserConstructionScript`)