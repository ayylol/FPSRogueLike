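; DoorCloseTrigger is a trigger actor that closes the door when the player overlaps it while it is active.
; On overlap it calls Close on the Door, deactivates itself and calls SetActive on the DoorTrigger, finding both through GetActorOfClass.
; Its own SetActive event re-arms it.
; The player check is an exact class match, and the lookups assume one Door and one DoorTrigger in the level.
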(event `self.ReceiveActorBeginOverlap`
  (params (OtherActor :type "Actor Object Reference"))
  (if (== (`GameplayStatics.GetObjectClass` OtherActor) "/Game/Blueprints/Player.Player_C")
    (if (`self.Active`)
      (bind _returnvalue (`GameplayStatics.GetActorOfClass` "/Game/Blueprints/Door.Door_C"))
      (`/Game/Blueprints/Door.Close` _returnvalue)
      (set `self.Active` false)
      (bind _returnvalue_2 (`GameplayStatics.GetActorOfClass` "/Game/Blueprints/Triggers/DoorTrigger.DoorTrigger_C"))
      (`/Game/Blueprints/Triggers/DoorTrigger.SetActive` _returnvalue_2))))

(event `SetActive`
  (set `self.Active` true))

(fn `UserConstructionScript`)