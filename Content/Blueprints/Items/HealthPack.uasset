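; HealthPack is an item Blueprint that gives the player health as its reward.
; Its Reward override runs the parent logic, then finds the GameMaster actor by class and adds a fixed amount to its PlayerHealth, with no clamp in this graph.
; The event graph holds only disabled default events, so whatever triggers Reward lives outside this file.
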(fn `Reward`
  (`parent.Reward`)
  (bind _returnvalue (`GameplayStatics.GetActorOfClass` "/Game/Blueprints/GameMaster.GameMaster_C"))
  (set `/Game/Blueprints/GameMaster.PlayerHealth` (+ (`/Game/Blueprints/GameMaster.PlayerHealth` _returnvalue) 10.0) _returnvalue))

(fn `UserConstructionScript`
  (`parent.UserConstructionScript`))