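; Placeholder actor Blueprint sketching a tabular Q-learning agent that is scored on an intensity value against a target.
; GetQ and SetQ treat a flat QTable array as a 2D state-action table, using NumOfRows as the stride per state.
; UpdateState advances to NextState, and Reward returns the signed difference between Intensity and TargetIntensity.
; SelectAction is empty, and no event or construction logic calls these helpers.
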(fn `GetQ`
  (params (State :type Integer) (Action :type Integer))
  (returns (QValue :type "Float (double-precision)"))
  (return (`|GetArrayItem` (`self.QTable`) (+ (* (`self.numOfRows`) State) Action))))

(fn `reward`
  (returns (Reward :type "Float (double-precision)"))
  (return (- (`self.Intensity`) (`self.targetIntensity`))))

(fn `SelectAction`)

(fn `SetQ`
  (params (State :type Integer) (Action :type Integer) (QValue :type "Float (double-precision)"))
  (`KismetArrayLibrary.Array_Set` (`self.QTable`) (+ (* (`self.numOfRows`) State) Action) QValue)
  (return))

(fn `updateState`
  (set `self.State` (`self.NextState`)))

(fn `UserConstructionScript`)