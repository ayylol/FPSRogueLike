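; NPC_ranged is a ranged enemy that attacks by firing EnemyProjectile actors.
; The Attack event sets an Attacking flag and starts a short one-shot timer, which spawns the projectile at the enemy's location and rotation, then clears the flag.
; The construction script runs the parent's script and sets this enemy's Health.
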(event `self.Attack`
  (set `self.Attacking` true)
  (`KismetSystemLibrary.K2_SetTimerDelegate` (delegate `CustomEvent_3`) 0.2))

(event `CustomEvent_3`
  (`|SpawnActorFromClass` "/Game/Blueprints/Weapons/EnemyProjectile.EnemyProjectile_C" (`KismetMathLibrary.MakeTransform` (`self.K2_GetActorLocation` self) (`self.K2_GetActorRotation` self)) "AlwaysSpawn" "OverrideRootScale" null null)
  (set `self.Attacking` false))

(fn `UserConstructionScript`
  (`parent.UserConstructionScript`)
  (set `self.Health` 11))