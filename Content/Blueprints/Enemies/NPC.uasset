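; NPC is an enemy character that takes shots, melee-attacks the player and can drop pickups when killed.
; Shot subtracts the GameMaster's damage value from Health, then at zero disables the capsule and delays Death by a timer.
; Death notifies GameMaster of the kill, rolls a rare DamageUp or occasional HealthPack drop, then destroys the actor.
; Attack uses timers to briefly enable WeaponBox collision, whose overlap damages the player.
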(event `Shot`
  (bind _health (`self.Health`))
  (bind _returnvalue (`GameplayStatics.GetActorOfClass` "/Game/Blueprints/GameMaster.GameMaster_C"))
  (if (> _health 0)
    (bind _output_get (set `self.Health` (- _health (`/Game/Blueprints/GameMaster.DamageToDeal` _returnvalue))))
    (if (<= _output_get 0)
      (set `self.Dying` true)
      (`PrimitiveComponent.SetCollisionEnabled` (`self.CapsuleComponent`) "NoCollision")
      (`KismetSystemLibrary.K2_SetTimerDelegate` (delegate `Death`) (`self.DeathTime`)))))

(event `Death`
  (bind _returnvalue (`KismetMathLibrary.RandomIntegerInRange` 0 100))
  (bind _returnvalue_2 (`KismetMathLibrary.MakeTransform` (`self.K2_GetActorLocation`)))
  (bind _returnvalue_3 (`GameplayStatics.GetActorOfClass` "/Game/Blueprints/GameMaster.GameMaster_C"))
  (`/Game/Blueprints/GameMaster.Enemykilled` _returnvalue_3)
  (if (< _returnvalue 2)
    (`|SpawnActorFromClass` "/Game/Blueprints/Items/DamageUp.DamageUp_C" _returnvalue_2 "Undefined" "OverrideRootScale" null null)
    (elif (< _returnvalue 12)
      (`|SpawnActorFromClass` "/Game/Blueprints/Items/HealthPack.HealthPack_C" _returnvalue_2 "Undefined" "OverrideRootScale" null null)))
  (`self.K2_DestroyActor`))

(event `Attack`
  (set `self.Attacking` true)
  (`KismetSystemLibrary.K2_SetTimerDelegate` (delegate `CustomEvent_0`) 0.2)
  (`KismetSystemLibrary.K2_SetTimerDelegate` (delegate `AttackEnd`) 0.8))

(event `AttackEnd`
  (set `self.Attacking` false))

(event `CustomEvent_0`
  (`PrimitiveComponent.SetCollisionEnabled` (`self.WeaponBox`) "QueryOnly")
  (`KismetSystemLibrary.K2_SetTimerDelegate` (delegate `CustomEvent_1`) 0.1))

(event `self.WeaponBox.OnComponentBeginOverlap`
  (params (OverlappedComponent :type "PrimitiveComponent Object Reference") (OtherActor :type "Actor Object Reference") (OtherComp :type "PrimitiveComponent Object Reference") (OtherBodyIndex :type Integer) (bFromSweep :type Boolean) (SweepResult :type "HitResult Structure (by ref)"))
  (if (== OtherActor (`GameplayStatics.GetPlayerCharacter` 0))
    (bind _asplayer (cast `/Game/Blueprints/Player` OtherActor))
    (`GameplayStatics.ApplyDamage` _asplayer (`self.DamageOut`) null self)))

(event `CustomEvent_1`
  (`PrimitiveComponent.SetCollisionEnabled` (`self.WeaponBox`) "NoCollision"))

(fn `UserConstructionScript`
  (set `self.DeathTime` 0.6))