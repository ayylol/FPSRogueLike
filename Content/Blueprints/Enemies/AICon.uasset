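; AI controller for enemy NPCs that picks a behavior tree and reports whether the player is perceived.
; On possess, it initializes the BasicNPCBlackboard, then runs RangedNPCTree for NPC_ranged pawns and BasicNPCTree for all others.
; AI Perception updates from the player character write the sensed state to the SeePlayer blackboard key.
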(event `self.ReceivePossess`
  (params (PossessedPawn :type "Pawn Object Reference"))
  (bind _blackboardcomponent (`self.UseBlackboard` "/Game/Blueprints/Enemies/BasicNPCBlackboard.BasicNPCBlackboard"))
  (set `self.Blackboard Component` _blackboardcomponent)
  (if (== (`GameplayStatics.GetObjectClass` PossessedPawn) "/Game/Blueprints/Enemies/NPC_ranged.NPC_ranged_C")
    (`self.RunBehaviorTree` "/Game/Blueprints/Enemies/RangedNPCTree.RangedNPCTree")
    (else
      (`self.RunBehaviorTree` "/Game/Blueprints/Enemies/BasicNPCTree.BasicNPCTree")))
  (`KismetSystemLibrary.PrintString` "Pssesed"))

(event `self.AIPerception.OnTargetPerceptionUpdated`
  (params (Actor :type "Actor Object Reference") (Stimulus :type "AIStimulus Structure"))
  (if (== Actor (`GameplayStatics.GetPlayerCharacter` 0))
    (`BlackboardComponent.SetValueAsBool` (`self.Blackboard Component`) (`KismetStringLibrary.Conv_StringToName` "SeePlayer") (`.bSuccessfullySensed` (break `AIStimulus` Stimulus)))))

(fn `UserConstructionScript`)