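; Behavior tree task that makes an NPC turn toward the player and perform its attack, named for ranged enemies.
; It fails immediately if the player is beyond a fixed distance from the controlled NPC.
; Otherwise a self-rescheduling timer lerps the capsule's yaw toward the player over about one second, using a plain float lerp from the current yaw.
; When the turn completes, it calls Attack on the NPC and finishes successfully.
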(event `self.ReceiveExecuteAI`
  (params (OwnerController :type "AIController Object Reference") (ControlledPawn :type "Pawn Object Reference"))
  (set `self.turn` 0.0)
  (bind _asnpc (cast `/Game/Blueprints/Enemies/NPC` ControlledPawn))
  (if (<= (`KismetMathLibrary.Vector_Distance` (`Actor.K2_GetActorLocation` _asnpc) (`Actor.K2_GetActorLocation` (`GameplayStatics.GetPlayerCharacter` 0))) 2000.0)
    (`KismetSystemLibrary.K2_SetTimerDelegate` (delegate `TurnEvent`) (`self.Turntime`))
    (else
      (`self.FinishExecute` false))))

(event `TurnEvent`
  (bind _output_get (set `self.turn` (+ (`self.turn`) (`self.Turntime`))))
  (bind _capsulecomponent (`Character.CapsuleComponent` (stale `self.ReceiveExecuteAI` _asnpc)))
  (`SceneComponent.K2_SetWorldRotation` _capsulecomponent (`KismetMathLibrary.MakeRotator` (.roll (`SceneComponent.K2_GetComponentRotation` _capsulecomponent)) (.pitch (`SceneComponent.K2_GetComponentRotation` _capsulecomponent)) (`KismetMathLibrary.Lerp` (.yaw (`SceneComponent.K2_GetComponentRotation` _capsulecomponent)) (.yaw (`KismetMathLibrary.FindLookAtRotation` (`SceneComponent.K2_GetComponentLocation` _capsulecomponent) (`SceneComponent.K2_GetComponentLocation` (`Character.CapsuleComponent` (`GameplayStatics.GetPlayerCharacter` 0))))) _output_get)) false false)
  (if (< _output_get 1.0)
    (`KismetSystemLibrary.K2_SetTimerDelegate` (delegate `TurnEvent`) (`self.Turntime`))
    (else
      (`/Game/Blueprints/Enemies/NPC.Attack` (stale `self.ReceiveExecuteAI` _asnpc))
      (`self.FinishExecute` true))))