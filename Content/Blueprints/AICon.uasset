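; AI controller that drives a basic NPC and tracks whether it can perceive the player.
; On possession it initializes the BasicNPC blackboard, runs the BasicNPC behavior tree and prints a debug string.
; AI Perception target updates for the player character write the sensed state to the SeePlayer blackboard bool.
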(event `self.ReceivePossess`
  (params (PossessedPawn :type "Pawn Object Reference"))
  (bind _blackboardcomponent (`self.UseBlackboard` "/Game/Blueprints/BasicNPCBlackboard.BasicNPCBlackboard"))
  (set `self.Blackboard Component` _blackboardcomponent)
  (`self.RunBehaviorTree` "/Game/Blueprints/BasicNPCTree.BasicNPCTree")
  (`KismetSystemLibrary.PrintString` "Pssesed"))

(event `self.AIPerception.OnTargetPerceptionUpdated`
  (params (Actor :type "Actor Object Reference") (Stimulus :type "AIStimulus Structure"))
  (if (== Actor (`GameplayStatics.GetPlayerCharacter` 0))
    (`BlackboardComponent.SetValueAsBool` (`self.Blackboard Component`) (`KismetStringLibrary.Conv_StringToName` "SeePlayer") (`.bSuccessfullySensed` (break `AIStimulus` Stimulus)))))

(fn `UserConstructionScript`)